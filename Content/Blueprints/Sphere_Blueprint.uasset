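; Sphere_Blueprint is an extra-life pickup for BP_HoppingCharacter, triggered by overlap on its Sphere component.
; When that character class overlaps, it raises CurrentHealth by one only if the value is exactly 1, then destroys itself whether or not health changed.
; Debug strings print on every overlap and on a successful health increase.
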(event OnComponentBeginOverlap(Sphere)
  (params (OverlappedComponent :type Primitive%20Component%20Object%20Reference) (OtherActor :type Actor%20Object%20Reference) (OtherComp :type Primitive%20Component%20Object%20Reference) (OtherBodyIndex :type Integer) (bFromSweep :type Boolean) (SweepResult :type Hit%20Result%20Structure%20%28by%20ref%29))
  (Development|PrintString "Lifeup")
  (if (Utilities|ClassIsChildOf (Utilities|GetClass OtherActor) "/Game/Blueprints/BP_HoppingCharacter.BP_HoppingCharacter_C")
    (Utilities|FlowControl|Sequence
      (:then_0
        (bind _asbp_hopping_character (Utilities|Casting|CastToBP_HoppingCharacter OtherActor))
        (if (== (Variables|/Game/Blueprints/BP_HoppingCharacter.BP_HoppingCharacter_C|GetCurrentHealth _asbp_hopping_character) 1)
          (Variables|/Game/Blueprints/BP_HoppingCharacter.BP_HoppingCharacter_C|SetCurrentHealth _asbp_hopping_character (+ (Variables|/Game/Blueprints/BP_HoppingCharacter.BP_HoppingCharacter_C|GetCurrentHealth _asbp_hopping_character) 1))
          (Development|PrintString "Life = 2")))
      (:then_1
        (Actor|DestroyActor)))))

(event Collision|EventActorBeginOverlap
  (params (OtherActor :type Actor%20Object%20Reference)))

(event EventTick
  (params (DeltaSeconds :type Float%20%28single-precision%29)))

(fn ConstructionScript)