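; TruckObstacleRight is a truck obstacle that slides along +Y and damages actors it overlaps in a hopping-character game.
; A bound ObstacleSpawn event starts a timeline that lerps it from its current location across a fixed distance without sweeping.
; Overlap applies damage to damageable actors, destroying the truck if a BP_HoppingCharacter's health then equals one.
; It also destroys itself on GameReset or when its Tick-accumulated lifetime expires.
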(event OnComponentBeginOverlap(StaticMeshComponent)
  (params (OverlappedComponent :type Primitive%20Component%20Object%20Reference) (OtherActor :type Actor%20Object%20Reference) (OtherComp :type Primitive%20Component%20Object%20Reference) (OtherBodyIndex :type Integer) (bFromSweep :type Boolean) (SweepResult :type Hit%20Result%20Structure%20%28by%20ref%29))
  ;[1 1 1] Damage
  (if (Variables|/Script/Engine.Actor|GetbCanBeDamaged OtherActor)
    (Game|Damage|ApplyDamage OtherActor 1.0 0 self)
    (bind _asbp_hopping_character (Utilities|Casting|CastToBP_HoppingCharacter OtherActor))
    (if (== (Variables|/Game/Blueprints/BP_HoppingCharacter.BP_HoppingCharacter_C|GetCurrentHealth _asbp_hopping_character) 1)
      (Actor|DestroyActor))))

(event Custom|ObstacleSpawn_Event
  ;[1 1 1] Spawn and Movement
  (Variables|Default|SetMovementVector (Transformation|GetActorLocation))
  (bind _left_right (Timeline|Move Play)
    (:Update
      (Transformation|SetActorLocation (Math|Vector|Lerp(Vector) (Variables|Default|GetMovementVector) (+ (Variables|Default|GetMovementVector) "0.000000,3000.000000,0.000000") _left_right) false false))))

(event Custom|GameReset_Event
  ;[1 1 1] Events
  (Actor|DestroyActor))

(event EventTick
  (params (DeltaSeconds :type Float%20%28single-precision%29))
  ;[1 1 1] Destroy
  (bind _output_get (Variables|Default|SetCurrent%20Lifetime (+ DeltaSeconds (Variables|Default|GetCurrent%20Lifetime))))
  (if (>= _output_get (Variables|Default|GetLifetime))
    (Actor|DestroyActor)))

(event EventBeginPlay
  ;[1 1 1] Events
  (Utilities|FlowControl|Sequence
    (:then_0
      (EventDispatchers|BindEventtoGameReset (delegate Custom|GameReset_Event)))
    (:then_1
      (EventDispatchers|BindEventtoObstacleSpawn (delegate Custom|ObstacleSpawn_Event)))))

(fn ConstructionScript)