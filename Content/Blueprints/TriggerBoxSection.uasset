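; Trigger box section that spawns left-side truck obstacles when a BP_HoppingCharacter overlaps it.
; The overlap destroys the Box component, spawns TruckObstacleLEft at a fixed offset from the actor and calls its CallObstacleSpawn.
; Spawning repeats after random delays until a check finds the player pawn beyond a set distance.
; A "Left" debug print fires on any overlap, and the other graphs are empty.
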(event OnComponentBeginOverlap(Box)
  (params (OverlappedComponent :type Primitive%20Component%20Object%20Reference) (OtherActor :type Actor%20Object%20Reference) (OtherComp :type Primitive%20Component%20Object%20Reference) (OtherBodyIndex :type Integer) (bFromSweep :type Boolean) (SweepResult :type Hit%20Result%20Structure%20%28by%20ref%29))
  (Development|PrintString "Left")
  (if (Utilities|ClassIsChildOf (Utilities|GetClass OtherActor) "/Game/Blueprints/BP_HoppingCharacter.BP_HoppingCharacter_C")
    (Components|DestroyComponent (Variables|Default|GetBox))
    (bind _returnvalue (Game|SpawnActorfromClass "/Game/Blueprints/TruckObstacleLEft.TruckObstacleLEft_C" (Math|Transform|MakeTransform (+ (Transformation|GetActorLocation) "600.000000,800.000000,0.000000")) "Undefined" "MultiplyWithRoot" 0 0 :!label _label))
    (Default|CallObstacleSpawn _returnvalue)
    (Utilities|FlowControl|Delay (Math|Random|RandomFloatinRange 1.2 3.0))
    (if (<= (Math|Vector|Distance(Vector) (Transformation|GetActorLocation self) (Transformation|GetActorLocation (Game|Player|GetPlayerPawn 0))) 8e+02)
      (goto _label))))

(fn ConstructionScript)

(fn NewFunction)